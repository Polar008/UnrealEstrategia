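; Tower defense game manager that runs the match: money, lives, turret purchases, enemy waves and level reset.
; BeginPlay enables mouse input, builds the tower list, creates the HUD and hidden reset screen, and caches Ruta spline actors.
; A Delay on Tick paces Powta spawns at random route ends, shortening the interval each spawn.
; PlaceTurret spawns affordable turrets at the deprojected cursor; Die reduces HP until the reset screen replaces the HUD.
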(event `self.ReceiveBeginPlay`
  (`KismetSystemLibrary.ExecuteConsoleCommand` "viewmode unlit" null)
  (`self.PlayerControllerVarSetter`)
  (`self.MakeStructureList`)
  (`self.CreateUI`)
  (`self.SaveSplines`)
  (`/Game/Blueprints/HUD.ChangeText` (`self.HUD`) 10))

(event `self.ReceiveTick`
  (params (DeltaSeconds :type "Float (single-precision)"))
  (`KismetSystemLibrary.Delay` (`self.DelaySpawn`))
  (`self.SpawnMob`)
  (`self.GetHarder`))

(fn `AddStonks`
  (params (toAdd :type Integer))
  (bind _output_get (set `self.Stonks` (+ toAdd (`self.Stonks`))))
  (`/Game/Blueprints/HUD.CHangeStonks` (`self.HUD`) _output_get))

(fn `CreateUI`
  (bind _returnvalue (`GameplayStatics.GetPlayerController` 0))
  (`/Engine/EditorBlueprintResources/StandardMacros.IsValid` (`self.HUD`)
    (:`Is Not Valid`
      (bind _returnvalue_2 (`|CreateWidget` "/Game/Blueprints/HUD.HUD_C" _returnvalue))
      (bind _output_get (set `self.HUD` _returnvalue_2))
      (`UserWidget.AddToViewport` _output_get 0)
      (bind _returnvalue_3 (`|CreateWidget` "/Game/Blueprints/REsetHUD.REsetHUD_C" _returnvalue))
      (bind _output_get_2 (set `self.ResetHUD` _returnvalue_3))
      (`UserWidget.AddToViewport` _output_get_2 0)
      (`Widget.SetVisibility` _returnvalue_3 "Hidden"))))

(fn `Die`
  (bind _returnvalue (- (`self.Hp`) 1))
  (if (> _returnvalue 1)
    (bind _output_get (set `self.Hp` _returnvalue))
    (`/Game/Blueprints/HUD.ChangeText` (`self.HUD`) _output_get)
    (else
      (`Widget.SetVisibility` (`self.ResetHUD`) "Visible")
      (`Widget.SetVisibility` (`self.HUD`) "Hidden"))))

(fn `GetHarder`
  (if (>= (- (`self.DelaySpawn`) 0.01) 0.0)
    (set `self.DelaySpawn` (- (`self.DelaySpawn`) 0.01))))

(fn `MakeStructureList`
  (bind _returnvalue (`AddComponent|NODE_AddBaseTower-0`))
  (`KismetArrayLibrary.Array_Add` (`self.StructureList`) _returnvalue)
  (bind _returnvalue_2 (`AddComponent|NODE_AddBetterTower-0`))
  (`KismetArrayLibrary.Array_Add` (`self.StructureList`) _returnvalue_2))

(fn `Place Turret`
  (params (Structure :type "/Game/Data/StructureData Object Reference"))
  (bind _returnvalue (`GameplayStatics.GetPlayerController` 0))
  (bind (_locationx _locationy) (`PlayerController.GetMousePosition` _returnvalue))
  (bind _returnvalue_2 (- (`self.Stonks`) (`/Game/Data/StructureData.Cost` Structure)))
  (bind _worldposition (`GameplayStatics.DeprojectScreenToWorld` _returnvalue (`KismetMathLibrary.MakeVector2D` _locationx _locationy)))
  (if (>= _returnvalue_2 0)
    (bind _output_get (set `self.Stonks` _returnvalue_2))
    (`/Game/Blueprints/HUD.CHangeStonks` (`self.HUD`) _output_get)
    (bind _returnvalue_3 (`|SpawnActorFromClass` "/Game/Blueprints/Cano.Cano_C" (`KismetMathLibrary.MakeTransform` (`KismetMathLibrary.MakeVector` (.x _worldposition) 1.0 (.z _worldposition))) "Undefined" "OverrideRootScale" null null))
    (bind _output_get_2 (set `self.Cano` _returnvalue_3))
    (`/Game/Blueprints/Cano.StatAdd` _output_get_2 (`/Game/Data/StructureData.Color` Structure))
    (`SceneComponent.SetRelativeScale3D` (`/Game/Blueprints/Cano.EnemyCol` (`self.Cano`)) (`KismetMathLibrary.Conv_DoubleToVector` (`/Game/Data/StructureData.Range` Structure)))
    (set `/Game/Blueprints/Cano.Firerate` (`/Game/Data/StructureData.Firerate` Structure) (`self.Cano`))))

(fn `PlayerControllerVarSetter`
  (bind _returnvalue (`GameplayStatics.GetPlayerController` 0))
  (set `PlayerController.bShowMouseCursor` true _returnvalue)
  (set `PlayerController.bEnableClickEvents` true _returnvalue)
  (set `PlayerController.bEnableMouseOverEvents` true _returnvalue)
  (set `PlayerController.bEnableTouchOverEvents` true _returnvalue))

(fn `Reset`
  (bind _returnvalue (`GameplayStatics.GetCurrentLevelName` true))
  (`GameplayStatics.OpenLevel` (`KismetStringLibrary.Conv_StringToName` _returnvalue)))

(fn `SaveSplines`
  (bind _outactors (`GameplayStatics.GetAllActorsOfClass` "/Game/Blueprints/Ruta.Ruta_C"))
  (set `self.Rutas` _outactors))

(fn `SpawnMob`
  (bind _outitem (`KismetArrayLibrary.Array_Random` (`self.Rutas`)))
  (bind _ruta (`/Game/Blueprints/Ruta.Ruta` _outitem))
  (bind _returnvalue (`|SpawnActorFromClass` "/Game/Blueprints/Powta.Powta_C" (`SplineComponent.GetTransformAtDistanceAlongSpline` _ruta (`SplineComponent.GetSplineLength` _ruta) "World" false) "Undefined" "OverrideRootScale" null null))
  (set `/Game/Blueprints/Powta.Spline` _outitem _returnvalue))

(fn `StopCanonMove`
  (`/Game/Blueprints/Cano.StopMove` (`self.Cano`)))

(fn `UserConstructionScript`)