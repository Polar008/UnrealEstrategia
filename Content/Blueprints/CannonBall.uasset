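; CannonBall is a homing projectile that chases its EnemyToKill target.
; Each tick it rotates toward the target and steps one unit along that direction without sweep or delta-time scaling, destroying itself if the target is invalid.
; When its Box overlaps any Powta actor, it adds one Stonks through the GMBBP game mode, then destroys both that actor and itself.
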(event `self.Box.OnComponentBeginOverlap`
  (params (OverlappedComponent :type "PrimitiveComponent Object Reference") (OtherActor :type "Actor Object Reference") (OtherComp :type "PrimitiveComponent Object Reference") (OtherBodyIndex :type Integer) (bFromSweep :type Boolean) (SweepResult :type "HitResult Structure (by ref)"))
  (bind _aspowta (cast `/Game/Blueprints/Powta` OtherActor))
  (bind _asgmbbp (cast `/Game/Blueprints/GMBBP` (`GameplayStatics.GetGameMode`)))
  (`/Game/Blueprints/GMBBP.AddStonks` _asgmbbp 1)
  (`self.K2_DestroyActor` _aspowta)
  (`self.K2_DestroyActor`))

(event `self.ReceiveTick`
  (params (DeltaSeconds :type "Float (single-precision)"))
  (bind _defaultsceneroot (`self.DefaultSceneRoot`))
  (bind _returnvalue (`SceneComponent.K2_GetComponentLocation` _defaultsceneroot))
  (bind _returnvalue_2 (`KismetMathLibrary.FindLookAtRotation` _returnvalue (`SceneComponent.K2_GetComponentLocation` (`/Game/Blueprints/Powta.DefaultSceneRoot` (`self.EnemyToKill`)))))
  (if (`KismetSystemLibrary.IsValid` (`self.EnemyToKill`))
    (`SceneComponent.K2_SetWorldRotation` _defaultsceneroot _returnvalue_2 false false)
    (`SceneComponent.K2_SetWorldLocation` (`self.DefaultSceneRoot`) (+ _returnvalue (`KismetMathLibrary.GetForwardVector` _returnvalue_2)) false false)
    (else
      (`self.K2_DestroyActor`))))

(fn `UserConstructionScript`)