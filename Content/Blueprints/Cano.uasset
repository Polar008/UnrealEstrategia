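; Cano is a placeable 2D cannon turret that shoots at Powta enemies in range.
; Until StopMove sets IsPlaced, it follows the mouse in the XZ plane; afterwards its barrel rotates toward the first tracked enemy.
; EnemyCol overlaps append enemies to a queue and drop the oldest entry on exit.
; A Delay on Tick paces Shoot, which spawns a CannonBall targeting that first enemy; StatAdd tints both sprites.
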(event `self.ReceiveTick`
  (params (DeltaSeconds :type "Float (single-precision)"))
  (`self.move`)
  (`KismetSystemLibrary.Delay` (`self.Firerate`))
  (`self.Shoot`))

(event `self.EnemyCol.OnComponentBeginOverlap`
  (params (OverlappedComponent :type "PrimitiveComponent Object Reference") (OtherActor :type "Actor Object Reference") (OtherComp :type "PrimitiveComponent Object Reference") (OtherBodyIndex :type Integer) (bFromSweep :type Boolean) (SweepResult :type "HitResult Structure (by ref)"))
  (bind _aspowta (cast `/Game/Blueprints/Powta` OtherActor))
  (`KismetArrayLibrary.Array_Add` (`self.Enemies`) _aspowta)
  (`KismetSystemLibrary.PrintString` "In"))

(event `self.EnemyCol.OnComponentEndOverlap`
  (params (OverlappedComponent :type "PrimitiveComponent Object Reference") (OtherActor :type "Actor Object Reference") (OtherComp :type "PrimitiveComponent Object Reference") (OtherBodyIndex :type Integer))
  (cast `/Game/Blueprints/Powta` OtherActor)
  (`KismetArrayLibrary.Array_Remove` (`self.Enemies`))
  (`KismetSystemLibrary.PrintString` "Out"))

(fn `move`
  (bind _returnvalue (`GameplayStatics.GetPlayerController` 0))
  (bind _enemies (`self.Enemies`))
  (bind _base (`self.Base`))
  (bind (_locationx _locationy) (`PlayerController.GetMousePosition` _returnvalue))
  (bind (_returnvalue_roll _returnvalue_pitch _returnvalue_yaw) (`KismetMathLibrary.BreakRotator` (`KismetMathLibrary.FindLookAtRotation` (`SceneComponent.K2_GetComponentLocation` _base) (`self.K2_GetActorLocation` (`|GetArrayItem` _enemies)))))
  (bind _worldposition (`GameplayStatics.DeprojectScreenToWorld` _returnvalue (`KismetMathLibrary.MakeVector2D` _locationx _locationy)))
  (if (`self.IsPlaced`)
    ;[0.1036 1 0] LookAt
    (if (> (`KismetArrayLibrary.Array_Length` _enemies) 0)
      (`/Engine/EditorBlueprintResources/StandardMacros.IsValid` _base
        (:`Is Valid`
          (`SceneComponent.K2_SetWorldRotation` (`self.Cano`) (`KismetMathLibrary.MakeRotator` _returnvalue_roll (+ _returnvalue_pitch -90.0) _returnvalue_yaw) false false))))
    (else
      (`SceneComponent.K2_SetWorldLocation` (`self.DefaultSceneRoot`) (`KismetMathLibrary.MakeVector` (.x _worldposition) 1.0 (.z _worldposition)) false false))))

(fn `Shoot`
  (if (and (> (`KismetArrayLibrary.Array_Length` (`self.Enemies`)) 0) (`self.IsPlaced`))
    (bind _returnvalue (`|SpawnActorFromClass` "/Game/Blueprints/CannonBall.CannonBall_C" (`SceneComponent.K2_GetComponentToWorld` (`self.Cano`)) "Undefined" "OverrideRootScale" null null))
    (`SceneComponent.K2_SetWorldRotation` :`self` (`Actor.RootComponent` _returnvalue))
    (set `/Game/Blueprints/CannonBall.EnemyToKill` (`|GetArrayItem` (`self.Enemies`)) _returnvalue)))

(fn `StatAdd`
  (params (color :type "Color Structure"))
  (bind _returnvalue (`KismetMathLibrary.Conv_ColorToLinearColor` color))
  (`PaperSpriteComponent.SetSpriteColor` (`self.Cano`) _returnvalue)
  (`PaperSpriteComponent.SetSpriteColor` (`self.Base`) _returnvalue))

(fn `StopMove`
  (set `self.IsPlaced` true))

(fn `UserConstructionScript`)