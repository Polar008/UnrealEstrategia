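; Powta is an actor that travels along a referenced spline and calls Die on the GMBBP game mode when it reaches the end of its run, then destroys itself.
; Tick caches the game mode and, while the spline is valid, plays a timeline with a rate scaled by Speed.
; The timeline moves it from the spline's far end back to its start, taking X and Z from the path and Y from Altura.
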(event `self.ReceiveTick`
  (params (DeltaSeconds :type "Float (single-precision)"))
  (bind _ruta (`/Game/Blueprints/Ruta.Ruta` (`self.Spline`)))
  (bind _asgmbbp (cast `/Game/Blueprints/GMBBP` (`GameplayStatics.GetGameMode`)))
  (set `self.Gm` _asgmbbp)
  (`/Engine/EditorBlueprintResources/StandardMacros.IsValid` (`self.Spline`)
    (:`Is Valid`
      (`TimelineComponent.SetPlayRate` (`self.MoveTL`) (/ (`self.Speed`) 100.0))
      (bind (_direction _track1) (`Timeline|MoveTL`)
        (:`Update`
          (bind (_returnvalue_x _returnvalue_y _returnvalue_z) (`KismetMathLibrary.BreakVector` (`SplineComponent.GetLocationAtDistanceAlongSpline` _ruta (`KismetMathLibrary.Lerp` (`SplineComponent.GetSplineLength` _ruta) 0.0 _track1) "World")))
          (`self.K2_SetActorTransform` (`KismetMathLibrary.MakeTransform` (`KismetMathLibrary.MakeVector` _returnvalue_x (`self.altura`) _returnvalue_z))))
        (:`Finished`
          (`/Game/Blueprints/GMBBP.Die` (`self.Gm`))
          (`self.K2_DestroyActor`))))))

(fn `UserConstructionScript`)